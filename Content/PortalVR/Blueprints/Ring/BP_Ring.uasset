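; BP_Ring is an actor with a WBP_Ring widget component that shows a scoreboard of players and scores.
; On BeginPlay it caches the widget.
; AddScore forwards a player name and points to BP_FirstPersonGameMode's UpdateGameScore.
; UpdateScore clears the board and refills it, one text line per player pairing name with score.
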(event `self.ReceiveBeginPlay`
  (bind _aswbp_ring (cast `/Game/PortalVR/Widgets/Ring/WBP_Ring` (`WidgetComponent.GetWidget` (`self.Widget`))))
  (set `self.As WBP Ring` _aswbp_ring))

(event `self.AddScore`
  (params (playerName :type String) (points :type Integer))
  (bind _asbp_first_person_game_mode (cast `/Game/FirstPerson/Blueprints/BP_FirstPersonGameMode` (`GameplayStatics.GetGameMode`)))
  (`/Game/FirstPerson/Blueprints/BP_FirstPersonGameMode.UpdateGameScore` _asbp_first_person_game_mode playerName points))

(event `UpdateScore`
  (params (Players :type "Array of String (by ref)") (Scores :type "Array of Integer (by ref)"))
  (`/Game/PortalVR/Widgets/Ring/WBP_Ring.ScoreboardClear` (`self.As WBP Ring`))
  (for (_array_element _array_index) Players
    (`/Game/PortalVR/Widgets/Ring/WBP_Ring.ScorepoardFilling` (`self.As WBP Ring`) (`KismetStringLibrary.Concat_StrStr` _array_element " with score " (`KismetStringLibrary.Conv_IntToString` (`|GetArrayItem` Scores _array_index))))))

(fn `UserConstructionScript`)